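; ZombieBP is a zombie actor that removes itself when the game's difficulty is too low for it.
; A one-time check on the first Tick, gated by InitialTickCheck, finds the RCGameMode actor and destroys the zombie if its Difficulty is below the zombie's DifficultyIndex.
; A helper function, DistanceFromBlast, returns the distance from a given blast position to the zombie's location.
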(event EventBeginPlay)

(event EventTick
  (params (DeltaSeconds :type Float%20%28single-precision%29))
  (if (Variables|Default|GetinitialTickCheck)
    (bind _outactors (Actor|GetAllActorsOfClass "/Game/BPs/newRC/RCGameMode.RCGameMode_C"))
    (if (Utilities|IsValid (Utilities|Array|Get(acopy) _outactors))
      (bind _output_get (Variables|Default|SetGameModeRef (Utilities|Array|Get(acopy) _outactors)))
      ;[1 1 1] Destroy if difficulty is lower than this being
      (if (< (Variables|/Game/BPs/newRC/RCGameMode.RCGameMode_C|GetDifficulty _output_get) (Variables|Default|GetdifficultyIndex))
        (Variables|Default|SetinitialTickCheck false) ; Destroy
        (Actor|DestroyActor)
        (else
          (Variables|Default|SetinitialTickCheck false :!label _label) ; don'tDestroy
        ))
      (else
        (goto _label)))))

(fn ConstructionScript)

(fn DistancefromBlast
  (params (blastTransform :type Vector))
  (return (Math|Vector|Distance(Vector) blastTransform (.Location (Math|Transform|BreakTransform (Transformation|GetActorTransform))))))