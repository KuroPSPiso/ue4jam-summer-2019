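; carSalvaged_BP is a drivable RC car vehicle controlled by player 0 through input axes.
; On BeginPlay it enables input and assigns a render target to its scene capture component, providing a camera feed from the car.
; DriveForward and MoveRight feed throttle and steering into the vehicle movement component only while IsControllerActive is set, which SetControllerState toggles.
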(event EventBeginPlay
  (Input|EnableInput (Game|GetPlayerController 0))
  ;[1 1 1] Bind Texture
  (Variables|/Script/Engine.SceneCaptureComponent2D|SetTextureTarget (Variables|Default|GetSceneCaptureComponent2D) (Variables|Default|GetTextureTarget)))

(event Input|AxisEvents|InputAxisMoveRight
  (params (AxisValue :type Float%20%28single-precision%29))
  (if (Variables|Default|GetIsControllerActive)
    (Class|WheeledVehicleMovementComponent|SetSteeringInput (Variables|Default|GetVehicleMovement) AxisValue)))

(event Input|AxisEvents|InputAxisDriveForward
  (params (AxisValue :type Float%20%28single-precision%29))
  (if (Variables|Default|GetIsControllerActive)
    (Class|WheeledVehicleMovementComponent|SetThrottleInput (Variables|Default|GetVehicleMovement) AxisValue)))

(fn ConstructionScript)

(fn SetControllerState
  (params (State :type Boolean))
  (Variables|Default|SetIsControllerActive State))